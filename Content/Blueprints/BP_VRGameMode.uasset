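; VR game mode that hands out pre-placed pawns to players and configures them by player count.
; Two seconds after BeginPlay, each VR player controller possesses the next VRPawn, and the player count goes to BP_VRGameState.
; For three to five players, it assigns numbered right-hand materials and destroys surplus pawns at fixed indices.
; ChoosePlayerStart picks the PlayerStart whose tag matches the current player count.
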(event `self.ReceiveBeginPlay`
  (bind _out_actors (`self.Out Actors`))
  (bind _output (`|GetArrayItem` _out_actors 2))
  (bind _output_2 (`|GetArrayItem` _out_actors 3))
  (bind _handright (`/Game/VRTemplate/Blueprints/VRPawn.HandRight` _output))
  (bind _handright_2 (`/Game/VRTemplate/Blueprints/VRPawn.HandRight` (`|GetArrayItem` _out_actors)))
  (bind _handright_3 (`/Game/VRTemplate/Blueprints/VRPawn.HandRight` (`|GetArrayItem` _out_actors 1)))
  ;[1 1 1] Muestra el numero introducido en el txt correspondiente
  (`KismetSystemLibrary.Delay` 2.0)
  (bind _outactors (`GameplayStatics.GetAllActorsOfClass` "/Game/VRTemplate/Blueprints/VRPawn.VRPawn_C"))
  (bind _output_get (set `self.Out Actors` _outactors))
  (bind _outactors_2 (`GameplayStatics.GetAllActorsOfClass` "/Game/Blueprints/BP_VRPlayerController.BP_VRPlayerController_C"))
  (for (_array_element _array_index) _outactors_2
    (if (== _array_index 0)
      _
      (else
        _))
    (`Controller.Possess` _array_element (`|GetArrayItem` _output_get (`self.NewVar`)))
    (`/Engine/EditorBlueprintResources/StandardMacros.IncrementInt` (`self.NewVar`)
      (:`  `
        (`KismetSystemLibrary.PrintString` "Poseido" true true (struct :`G` 0.66 :`B` 1.0 :`A` 1.0) 50.0)
        (`KismetSystemLibrary.PrintString` (`KismetSystemLibrary.GetDisplayName` _array_element) true true (struct :`G` 0.66 :`B` 1.0 :`A` 1.0) 50.0))))
  (bind _returnvalue (`self.GetNumPlayers`))
  (bind _asbp_vrgame_state (cast `/Game/Blueprints/BP_VRGameState` (`GameplayStatics.GetGameState`)))
  (`/Game/Blueprints/BP_VRGameState.Postit` _asbp_vrgame_state _returnvalue)
  (if (not (== _returnvalue 1))
    (switch `int` _returnvalue
      (:`3`
        (`PrimitiveComponent.SetMaterial` _handright_2 0 "/Game/Characters/MannequinsXR/Materials/Instances/Manny/MI_Manny_N4.MI_Manny_N4")
        (`PrimitiveComponent.SetMaterial` _handright_3 0 "/Game/Characters/MannequinsXR/Materials/Instances/Manny/MI_Manny_N9.MI_Manny_N9")
        (`self.K2_DestroyActor` _output_2)
        (`self.K2_DestroyActor` _output))
      (:`4`
        (`PrimitiveComponent.SetMaterial` _handright_2 0 "/Game/Characters/MannequinsXR/Materials/Instances/Manny/MI_Manny_N8.MI_Manny_N8")
        (`PrimitiveComponent.SetMaterial` _handright_3 0 "/Game/Characters/MannequinsXR/Materials/Instances/Manny/MI_Manny_N4.MI_Manny_N4")
        (`PrimitiveComponent.SetMaterial` _handright 0 "/Game/Characters/MannequinsXR/Materials/Instances/Manny/MI_Manny_N9.MI_Manny_N9")
        (`self.K2_DestroyActor` _output_2))
      (:`5`
        (`PrimitiveComponent.SetMaterial` _handright_2 0 "/Game/Characters/MannequinsXR/Materials/Instances/Manny/MI_Manny_N3.MI_Manny_N3")
        (`PrimitiveComponent.SetMaterial` _handright_3 0 "/Game/Characters/MannequinsXR/Materials/Instances/Manny/MI_Manny_N8.MI_Manny_N8")
        (`PrimitiveComponent.SetMaterial` _handright 0 "/Game/Characters/MannequinsXR/Materials/Instances/Manny/MI_Manny_N4.MI_Manny_N4")
        (`PrimitiveComponent.SetMaterial` (`/Game/VRTemplate/Blueprints/VRPawn.HandRight` _output_2) 0 "/Game/Characters/MannequinsXR/Materials/Instances/Manny/MI_Manny_N9.MI_Manny_N9")))))

(fn `ChoosePlayerStart`
  (params (Player :type "Controller Object Reference"))
  (returns (ReturnValue :type "Actor Object Reference"))
  (bind _returnvalue (`self.GetNumPlayers`))
  (bind _outactors (`GameplayStatics.GetAllActorsOfClass` "/Script/Engine.PlayerStart"))
  (for _array_element _outactors
    (if (== _returnvalue (`KismetStringLibrary.Conv_NameToString` (`PlayerStart.PlayerStartTag` _array_element)))
      (return _array_element))))

(fn `UserConstructionScript`)