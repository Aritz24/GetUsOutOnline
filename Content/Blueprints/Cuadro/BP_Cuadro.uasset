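; VR painting actor (Cuadro) that swings on a hinge when grabbed, apparently covering a safe.
; GrabComponent grabs alternate through a FlipFlop between a timed opening rotation, run only the first time, and a closing one, with a door sound on each grab.
; The first grab also enables collisions on BP_CajaFuerte.
; Hand-tracked rotation in UpdateMovement, clamped by spline points, is left disconnected, though dropping still clears its timer.
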(event `self.GrabComponent.OnGrabbed`
  (params (`Motion Controller` :type "MotionControllerComponent Object Reference"))
  (`GameplayStatics.PlaySoundAtLocation` "/Game/Audio/Audio_PuertaAbriendose1Mitad.Audio_PuertaAbriendose1Mitad" (`self.K2_GetActorLocation`) (struct) 1.0 1.0 0.0 null null null null)
  (`/Engine/EditorBlueprintResources/StandardMacros.FlipFlop`
    (:`A`
      (if (not (`self.Habilitadas`))
        (bind _returnvalue (`GameplayStatics.GetActorOfClass` "/Game/Blueprints/CajaFuerte/BP_CajaFuerte/BP_CajaFuerte.BP_CajaFuerte_C"))
        (`/Game/Blueprints/CajaFuerte/BP_CajaFuerte/BP_CajaFuerte.HabilitarColisiones` _returnvalue)
        (set `self.Habilitadas` true)
        (set `self.RotacionZ` 160.0)
        (`KismetSystemLibrary.MoveComponentTo` (`self.Scene`) (0.0 0.0 0.0) (`KismetMathLibrary.MakeRotator` 0.0 0.0 (`self.RotacionZ`)) false false 2.0 :!label _label)))
    (:`B`
      (set `self.RotacionZ` 2.0)
      (goto _label))))

(event `self.GrabComponent.OnDropped`
  (`KismetSystemLibrary.K2_ClearAndInvalidateTimerHandle` (`self.Timer`))
  (set `self.Motion Controller` null))

(fn `UpdateMovement`
  (locals (NewLocalVar :type "Float (double-precision)" :default 0.0))
  (bind _spline (`self.Spline`))
  (bind _capsule (`self.Capsule`))
  (bind _scene (`self.Scene`))
  (bind _returnvalue_x (`KismetMathLibrary.BreakVector` (`SplineComponent.GetLocationAtSplinePoint` _spline 1 "Local")))
  (bind _returnvalue_x_2 (`KismetMathLibrary.BreakVector` (`SplineComponent.GetLocationAtSplinePoint` _spline 0 "Local")))
  (bind (_relativerotation_roll _relativerotation_pitch _relativerotation_yaw) (`KismetMathLibrary.BreakRotator` (`SceneComponent.RelativeRotation` _scene)))
  (bind _returnvalue_location (`KismetMathLibrary.BreakTransform` (`KismetMathLibrary.MakeRelativeTransform` (`SceneComponent.K2_GetComponentToWorld` (`self.Motion Controller`)) (`SceneComponent.K2_GetComponentToWorld` _capsule))))
  (bind _returnvalue_x_3 (`KismetMathLibrary.BreakVector` (- (`SceneComponent.RelativeLocation` _capsule) _returnvalue_location)))
  (`SceneComponent.K2_SetRelativeRotation` _scene (`KismetMathLibrary.MakeRotator` _relativerotation_roll _relativerotation_pitch (`KismetMathLibrary.FClamp` (+ _relativerotation_yaw _returnvalue_x_3) _returnvalue_x_2 _returnvalue_x)) false false))

(fn `UserConstructionScript`)