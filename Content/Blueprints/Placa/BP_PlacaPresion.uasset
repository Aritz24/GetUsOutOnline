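; Pressure plate that sinks as its tracked weight grows, up to a limit set by PesoMaximo.
; Box overlap begin and end add or subtract OverlappedComponent's mass (the trigger itself, not the other component) and step the trigger up or down.
; Each change restarts a Timeline that lerps the platform from its current position toward the weight-based depth.
; Debug prints show weight and trigger location; several leftover trace and cast snippets never run.
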(event `self.ReceiveBeginPlay`
  ;[1 1 1] SetLocation
  (bind _output_get (set `self.StartLocation` (`SceneComponent.K2_GetComponentLocation` (`self.PlataformaPlaca`))))
  (set `self.CollisionLocation` (`SceneComponent.K2_GetComponentLocation` (`self.Box`)))
  (set `self.CurrentLocation` _output_get))

(event `self.Box.OnComponentBeginOverlap`
  (params (OverlappedComponent :type "PrimitiveComponent Object Reference") (OtherActor :type "Actor Object Reference") (OtherComp :type "PrimitiveComponent Object Reference") (OtherBodyIndex :type Integer) (bFromSweep :type Boolean) (SweepResult :type "HitResult Structure (by ref)"))
  (bind (_collisionlocation_x _collisionlocation_y _collisionlocation_z) (`KismetMathLibrary.BreakVector` (`self.CollisionLocation`)))
  (bind (_startlocation_x _startlocation_y _startlocation_z) (`KismetMathLibrary.BreakVector` (`self.StartLocation`)))
  (bind _returnvalue (+ _collisionlocation_z 15.0))
  ;[1 1 1] Overlap
  (bind _output_get (set `self.PesoEnPlaca` (+ (`PrimitiveComponent.GetMass` OverlappedComponent) (`self.PesoEnPlaca`))))
  (`KismetSystemLibrary.PrintString` (`KismetStringLibrary.Conv_IntToString` (`KismetMathLibrary.FTrunc` _output_get)) true true (struct :`R` 1.0 :`B` 0.056943 :`A` 1.0))
  (`SceneComponent.K2_SetWorldLocation` (`self.Box`) (`KismetMathLibrary.MakeVector` _collisionlocation_x _collisionlocation_y _returnvalue) false false)
  (bind _output_get_2 (set `self.CollisionLocation` (`KismetMathLibrary.MakeVector` _collisionlocation_x _collisionlocation_y _returnvalue)))
  (`KismetSystemLibrary.PrintString` (`KismetStringLibrary.Conv_VectorToString` _output_get_2))
  (bind _output_get_3 (set `self.EndLocation` (`KismetMathLibrary.MakeVector` _startlocation_x _startlocation_y (- _startlocation_z (* (`KismetMathLibrary.FClamp` (/ (`self.PesoEnPlaca`) (`self.PesoMaximo`))) 5.0)))))
  (bind (_direction _movimiento) (`Timeline|Timeline` :!via `PlayFromStart`)
    (:`Update`
      (bind _returnvalue_2 (`KismetMathLibrary.VLerp` (`self.CurrentLocation`) _output_get_3 _movimiento))
      (`SceneComponent.K2_SetWorldLocation` (`self.PlataformaPlaca`) _returnvalue_2 false false)
      (set `self.CurrentLocation` _returnvalue_2))))

(event `self.Box.OnComponentEndOverlap`
  (params (OverlappedComponent :type "PrimitiveComponent Object Reference") (OtherActor :type "Actor Object Reference") (OtherComp :type "PrimitiveComponent Object Reference") (OtherBodyIndex :type Integer))
  (bind (_collisionlocation_x _collisionlocation_y _collisionlocation_z) (`KismetMathLibrary.BreakVector` (`self.CollisionLocation`)))
  (bind (_startlocation_x _startlocation_y _startlocation_z) (`KismetMathLibrary.BreakVector` (`self.StartLocation`)))
  (bind _returnvalue (- _collisionlocation_z 15.0))
  ;[1 1 1] EndOverlp
  (bind _output_get (set `self.PesoEnPlaca` (- (`self.PesoEnPlaca`) (`PrimitiveComponent.GetMass` (stale `self.Box.OnComponentBeginOverlap` OverlappedComponent)))))
  (`KismetSystemLibrary.PrintString` (`KismetStringLibrary.Conv_IntToString` (`KismetMathLibrary.FTrunc` _output_get)) true true (struct :`R` 1.0 :`B` 0.204647 :`A` 1.0))
  (`SceneComponent.K2_SetWorldLocation` (`self.Box`) (`KismetMathLibrary.MakeVector` _collisionlocation_x _collisionlocation_y _returnvalue) false false)
  (set `self.CollisionLocation` (`KismetMathLibrary.MakeVector` _collisionlocation_x _collisionlocation_y _returnvalue))
  (bind _output_get_2 (set `self.EndLocation` (`KismetMathLibrary.MakeVector` _startlocation_x _startlocation_y (- _startlocation_z (* (`KismetMathLibrary.FClamp` (/ (`self.PesoEnPlaca`) (`self.PesoMaximo`))) 5.0)))))
  (bind (_direction _movimiento) (`Timeline|Timeline_0` :!via `PlayFromStart`)
    (:`Update`
      (bind _returnvalue_2 (`KismetMathLibrary.VLerp` (`self.CurrentLocation`) _output_get_2 _movimiento))
      (`SceneComponent.K2_SetWorldLocation` (`self.PlataformaPlaca`) _returnvalue_2 false false)
      (set `self.CurrentLocation` _returnvalue_2))))

(fn `UserConstructionScript`)