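; Lobby game mode that tracks joined players and their ready state, and server-travels everyone to the Main level.
; On login it gathers each BP_LobbyPlayerController's info, creates its menu widget and pushes the player list to all controllers.
; Status updates rebuild that list and enable the host's colored Start button when the ready count equals players minus one.
; ChoosePlayerStart picks the PlayerStart whose tag matches the current player count.
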(event `Server travel`
  ;[1 1 1] Takes all players to the play map
  (`KismetSystemLibrary.ExecuteConsoleCommand` "ServerTravel /Game/Levels/Main" (`GameplayStatics.GetPlayerController` 0)))

(event `self.K2_PostLogin`
  (params (NewPlayer :type "PlayerController Object Reference"))
  (bind _returnvalue (`self.GetNumPlayers`))
  (set `self.NumPlayers` _returnvalue)
  ;[1 1 1] Cada vez que entra un jugador actuliza la lista y le crea su widget de menu
  (bind _asbp_lobby_player_controller (cast `/Game/Blueprints/Lobby/Blueprint/BP_LobbyPlayerController` NewPlayer :!label _label)
    (:`then`
      (bind _output_get (set `self.As BP Lobby Player Controller` _asbp_lobby_player_controller))
      (`/Game/Blueprints/Lobby/Blueprint/BP_LobbyPlayerController.UpdatePlayerInfo` _asbp_lobby_player_controller)
      (`/Game/Blueprints/Lobby/Blueprint/BP_LobbyPlayerController.UpdatePlayerInfo` _output_get)
      (`KismetSystemLibrary.Delay` 0.2)
      (`KismetArrayLibrary.Array_Add` (`self.PlayerControllers`) _asbp_lobby_player_controller)
      (`KismetArrayLibrary.Array_Add` (`self.PlayerInfo`) (`/Game/Blueprints/Lobby/Blueprint/BP_LobbyPlayerController.PlayerInfo` (`self.As BP Lobby Player Controller`)))
      (`KismetSystemLibrary.Delay` 0.2)
      (`/Game/Blueprints/Lobby/Blueprint/BP_LobbyPlayerController.CreateWidget` _asbp_lobby_player_controller)
      (`self.UpdatePlayerList`))
    (:`CastFailed`
      ;[1 1 1] Takes all players to the play map
      (`KismetSystemLibrary.PrintString` "Hello"))))

(event `self.K2_OnLogout`
  (params (ExitingController :type "Controller Object Reference"))
  (bind _asbp_lobby_player_controller (cast `/Game/Blueprints/Lobby/Blueprint/BP_LobbyPlayerController` ExitingController))
  (`KismetArrayLibrary.Array_RemoveItem` (`self.PlayerControllers`) _asbp_lobby_player_controller)
  (goto _label))

(event `UpdatePlayerList`
  ;[1 1 1] Actualiza la lista de jugadores en la sesion
  (for _array_element (`self.PlayerControllers`)
    (`/Game/Blueprints/Lobby/Blueprint/BP_LobbyPlayerController.UpdatePlayerList` _array_element (`self.PlayerInfo`))))

(event `UpdateStatus`
  (bind _playercontrollers (`self.PlayerControllers`))
  ;[1 1 1] Limpia el array playerInfo y lo llena con datos actualizados
  (`KismetArrayLibrary.Array_Clear` (`self.PlayerInfo`))
  (for _array_element (`self.PlayerControllers`)
    (`KismetArrayLibrary.Array_Add` (`self.PlayerInfo`) (`/Game/Blueprints/Lobby/Blueprint/BP_LobbyPlayerController.PlayerInfo` _array_element)))
  (`KismetSystemLibrary.Delay` 0.2)
  ;[1 1 1] Comprueba si los jugadores están listos para jugar
  (set `self.PlayerCount` (- (`KismetArrayLibrary.Array_Length` _playercontrollers) 1))
  (for _array_element_2 _playercontrollers
    (bind _playerinfo_isready (break `/Game/Widgets/BlueprintsLobby/PlayerInfo` (`/Game/Blueprints/Lobby/Blueprint/BP_LobbyPlayerController.PlayerInfo` _array_element_2)))
    (if _playerinfo_isready
      (`/Engine/EditorBlueprintResources/StandardMacros.IncrementInt` (`self.PlayersReady`)
        (:`  `
          _)))
    (`/Game/Blueprints/Lobby/Blueprint/BP_LobbyPlayerController.UpdatePlayerList` _array_element_2 (`self.PlayerInfo`)))
  ;[1 1 1] Habilita o deshabilita el botón start dependiendo de si todos los jugadores están listos
  (bind _asbp_lobby_player_controller (cast `/Game/Blueprints/Lobby/Blueprint/BP_LobbyPlayerController` (`GameplayStatics.GetPlayerController` 0)))
  (bind _aswid_host_screen (cast `/Game/Widgets/WidgetsLobby/WID_HostScreen` (`/Game/Blueprints/Lobby/Blueprint/BP_LobbyPlayerController.LobbyWidget` _asbp_lobby_player_controller)))
  (`self.Habilitar/deshabilitarBotonStart` (`/Game/Widgets/WidgetsLobby/WID_HostScreen.btn_Start` _aswid_host_screen) (== (`self.PlayerCount`) (`self.PlayersReady`))))

(event `Habilitar/deshabilitarBotonStart`
  (params (Button :type "Button Object Reference") (`PlayerCount==Ready` :type Boolean))
  (if `PlayerCount==Ready`
    (set `Widget.bIsEnabled` true Button)
    (`Button.SetColorAndOpacity` Button (struct :`G` 1.0 :`B` 0.205079 :`A` 1.0))
    (else
      (set `Widget.bIsEnabled` false Button)
      (`Button.SetColorAndOpacity` Button (struct :`R` 1.0 :`B` 0.084376 :`A` 1.0))
      (set `self.PlayersReady` 0))))

(fn `ChoosePlayerStart`
  (params (Player :type "Controller Object Reference"))
  (returns (ReturnValue :type "Actor Object Reference"))
  (bind _returnvalue (`self.GetNumPlayers`))
  (bind _outactors (`GameplayStatics.GetAllActorsOfClass` "/Script/Engine.PlayerStart"))
  (for _array_element _outactors
    (if (== _returnvalue (`KismetStringLibrary.Conv_NameToString` (`PlayerStart.PlayerStartTag` _array_element)))
      (return _array_element))))

(fn `UserConstructionScript`)